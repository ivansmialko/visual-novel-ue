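; BP_DialogInstance tracks the current node of a branching dialog read from a DataTable.
; Initialize stores the table and marks the instance ready if it has rows; StartDialogFromBeginning then loads row "0" as the current node.
; ProvideReply validates the reply index, then advances through FindNodeById using the first reply's NextNodeId, whichever index was given.
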(fn `FindNodeById`
  (params (NodeId :type Name))
  (returns (FoundNode :type "/Game/_Code/Structs/Dialog/S_DialogNode Structure"))
  (if (`self.IsInitialized`)
    (bind _returnvalue (`|GetDataTableRow` (`self.CurrentDialogData`) NodeId)
      (:`then`
        _)
      (:`RowNotFound`
        _))
    (return _returnvalue)))

(fn `Initialize`
  (params (DialogDataTable :type "DataTable Object Reference"))
  (`/Engine/EditorBlueprintResources/StandardMacros.IsValid` DialogDataTable
    (:`Is Valid`
      (set `self.CurrentDialogData` DialogDataTable)
      (bind _outrownames (`DataTableFunctionLibrary.GetDataTableRowNames` (`self.CurrentDialogData`)))
      (if (!= (`KismetArrayLibrary.Array_Length` _outrownames) 0)
        (set `self.IsInitialized` true)))))

(fn `ProvideReply`
  (params (ReplyIndex :type Integer))
  (locals (LocalReplyIndex :type Integer))
  (bind (_currentdialognode_nodeid _currentdialognode_text _currentdialognode_replylist) (break `/Game/_Code/Structs/Dialog/S_DialogNode` (`self.CurrentDialogNode`)))
  (bind (_currentdialognode_nodeid_2 _currentdialognode_text_2 _currentdialognode_replylist_2) (break `/Game/_Code/Structs/Dialog/S_DialogNode` (`self.CurrentDialogNode`)))
  (set `local.LocalReplyIndex` ReplyIndex)
  (if (`KismetArrayLibrary.Array_IsValidIndex` _currentdialognode_replylist_2 (`local.LocalReplyIndex`))
    (bind _foundnode (`self.FindNodeById` (`KismetStringLibrary.Conv_StringToName` (`KismetStringLibrary.Conv_IntToString` (`.NextNodeId_6_6A17E3D14DA6D1E1D190DB87FA1A6FC4` (break `/Game/_Code/Structs/Dialog/S_DialogReply` (`|GetArrayItem` _currentdialognode_replylist)))))))
    (set `self.CurrentDialogNode` _foundnode)))

(fn `StartDialogFromBeginning`
  (if (`self.IsInitialized`)
    (bind _returnvalue (`|GetDataTableRow` (`self.CurrentDialogData`) "0")
      (:`then`
        (set `self.CurrentDialogNode` _returnvalue)))))