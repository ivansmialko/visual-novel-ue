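; BP_DialogManager is an actor that starts dialogs by ID and exposes the current dialog node.
; Initialize stores a dialog data table and constructs a single BP_DialogInstance that is reused for each dialog.
; StartDialog builds a row name from a "Dialog_" prefix and the ID, then hands that row's dialog reference to the instance and starts it from the beginning.
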(event `self.ReceiveBeginPlay`)

(fn `GetCurrentDialogNode`
  (returns (CurrentDialogNode :type "/Game/_Code/Structs/Dialog/S_DialogNode Structure"))
  (if (`self.IsInitialized`)
    (return (`/Game/_Code/Dialogs/BP_DialogInstance.CurrentDialogNode` (`self.CurrentDialogInstance`)))))

(fn `Initialize`
  (params (DialogsDataTable :type "DataTable Object Reference"))
  (`/Engine/EditorBlueprintResources/StandardMacros.IsValid` DialogsDataTable
    (:`Is Valid`
      (set `self.DialogsTable` DialogsDataTable)
      (bind _returnvalue (`|GenericCreateObject` "/Game/_Code/Dialogs/BP_DialogInstance.BP_DialogInstance_C"))
      (set `self.CurrentDialogInstance` _returnvalue)
      (set `self.IsInitialized` true))))

(fn `Start Dialog`
  (params (DialogId :type Integer))
  (locals (TargetDialogTableName :type String) (FoundDialogTableRow :type "/Game/_Code/Structs/Dialog/S_DialogsTableRow Structure"))
  (if (`self.IsInitialized`)
    (set `self.CurrentDialogId` DialogId)
    (bind _output_get (set `local.TargetDialogTableName` (`KismetStringLibrary.Concat_StrStr` "Dialog_" (`KismetStringLibrary.Conv_IntToString` (`self.CurrentDialogId`)))))
    (bind _returnvalue (`|GetDataTableRow` (`self.DialogsTable`) (`KismetStringLibrary.Conv_StringToName` _output_get))
      (:`then`
        (bind _output_get_2 (set `local.FoundDialogTableRow` _returnvalue))
        (bind _output_get_3 (set `self.CurrentDialog` (`.DialogReference_2_74D37E1540B8F76EF2CA52AD0E75DE43` (break `/Game/_Code/Structs/Dialog/S_DialogsTableRow` _output_get_2))))
        (`/Game/_Code/Dialogs/BP_DialogInstance.Initialize` (`self.CurrentDialogInstance`) _output_get_3)
        (`/Game/_Code/Dialogs/BP_DialogInstance.StartDialogFromBeginning` (`self.CurrentDialogInstance`))))))

(fn `UserConstructionScript`)