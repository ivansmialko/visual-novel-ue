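; BP_DialogMechanic is an actor that connects the dialog manager to the dialog UI.
; Initialize creates and shows W_DialogUI, passes it a self reference, and spawns a BP_DialogManager initialized with the DT_Dialogs data table.
; LaunchDialog starts a dialog by ID and InputReply forwards a chosen reply index; both then refresh the widget with the manager's current dialog node.
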(fn `Initialize`
  (`/Engine/EditorBlueprintResources/StandardMacros.IsValid` (`self.W_DialogUIRef`)
    (:`Is Valid`
      _)
    (:`Is Not Valid`
      (bind _returnvalue (`|CreateWidget` "/Game/_Code/UI/DIalogMechanics/W_DialogUI.W_DialogUI_C" (`GameplayStatics.GetPlayerController` 0)))
      (set `self.W_DialogUIRef` _returnvalue)))
  (`UserWidget.AddToViewport` (`self.W_DialogUIRef`) 0)
  (set `/Game/_Code/UI/DIalogMechanics/W_DialogUI.DialogMechanic` self (`self.W_DialogUIRef`))
  (`/Engine/EditorBlueprintResources/StandardMacros.IsValid` (`self.DialogManager`)
    (:`Is Valid`
      _)
    (:`Is Not Valid`
      (bind _returnvalue_2 (`|SpawnActorFromClass` "/Game/_Code/Dialogs/BP_DialogManager.BP_DialogManager_C" (`KismetMathLibrary.MakeTransform` (0.0 0.0 0.0)) "Undefined" "OverrideRootScale" null null))
      (bind _output_get (set `self.DialogManager` _returnvalue_2))))
  (`/Game/_Code/Dialogs/BP_DialogManager.Initialize` _output_get "/Game/_Assets/Dialogs/DT_Dialogs.DT_Dialogs"))

(fn `InputReply`
  (params (ReplyIndex :type Integer))
  (`/Game/_Code/Dialogs/BP_DialogManager.ProvideReply` (`self.DialogManager`) ReplyIndex)
  (`self.UpdateDialogUI`))

(fn `LaunchDialog`
  (params (DialogId :type Integer))
  (`/Game/_Code/Dialogs/BP_DialogManager.Start Dialog` (`self.DialogManager`) DialogId)
  (`self.UpdateDialogUI`))

(fn `UpdateDialogUI`
  (`/Game/_Code/UI/DIalogMechanics/W_DialogUI.Display Dialog Node` (`self.W_DialogUIRef`) (`/Game/_Code/Dialogs/BP_DialogManager.GetCurrentDialogNode` (`self.DialogManager`))))

(fn `UserConstructionScript`)